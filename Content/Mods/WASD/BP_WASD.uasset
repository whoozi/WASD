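; WASD mod Blueprint that adds camera-relative keyboard movement alongside the SetDestination input.
; Each tick it force-feeds a vector built from camera yaw and movement axes into player 0's CharacterMovement, turns control rotation to match and ignores normal move input.
; Movement is blocked during montages unless they pass section, play-rate and name-prefix checks.
; Pressing or releasing SetDestination without WASD input restores normal move input.
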(event `self.ReceiveTick`
  (params (DeltaSeconds :type "Float (single-precision)"))
  (bind _returnvalue (`GameplayStatics.GetPlayerController` 0))
  (bind (_returnvalue_roll _returnvalue_pitch _returnvalue_yaw) (`KismetMathLibrary.BreakRotator` (`PlayerCameraManager.GetCameraRotation` (`GameplayStatics.GetPlayerCameraManager` 0))))
  (bind _returnvalue_2 (`SkeletalMeshComponent.GetAnimInstance` (`Character.Mesh` (`GameplayStatics.GetPlayerCharacter` 0))))
  (bind _returnvalue_3 (`KismetMathLibrary.MakeRotator` _returnvalue_roll 0.0 _returnvalue_yaw))
  (bind _returnvalue_4 (`AnimInstance.IsAnyMontagePlaying` _returnvalue_2))
  (bind _returnvalue_5 (+ (* (`KismetMathLibrary.GetForwardVector` _returnvalue_3) (`self.GetInputAxisValue`)) (* (`KismetMathLibrary.GetRightVector` _returnvalue_3) (`self.GetInputAxisValue`))))
  (if (and (`self.Is WASD Input`) (or (not _returnvalue_4) (and _returnvalue_4 (`self.Can Move During Montage` _returnvalue_2 (`AnimInstance.GetCurrentActiveMontage` _returnvalue_2)))))
    (`PawnMovementComponent.AddInputVector` (`Character.CharacterMovement` (`GameplayStatics.GetPlayerCharacter` 0)) _returnvalue_5 true)
    (`Controller.SetControlRotation` _returnvalue (`KismetMathLibrary.Conv_VectorToRotator` _returnvalue_5))
    (`Controller.SetIgnoreMoveInput` _returnvalue true)))

(event `InputAction|SetDestination` :consume false
  (params (Key :type "Key Structure"))
  (:`Pressed`
    (if (not (`self.Is WASD Input`)) :!label _label
      (`Controller.ResetIgnoreMoveInput` (`GameplayStatics.GetPlayerController` 0))))
  (:`Released`
    (goto _label)))

(fn `UserConstructionScript`)